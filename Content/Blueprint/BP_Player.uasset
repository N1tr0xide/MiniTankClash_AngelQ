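; Player blueprint that drives a BP-TankBase child actor, using its camera and a HUD showing health and remaining enemies from GM_Main.
; Enhanced Input feeds throttle, steering and clamped spring-arm look to the tank.
; Each tick the upper body follows the spring arm and the cannon pitches toward screen center.
; Shooting uses the tank's cannon cast, delaying tank damage by distance over bullet speed, or spawning dirt blasts on other hits.
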(event `self.ReceiveBeginPlay`
  (bind _returnvalue (`GameplayStatics.GetPlayerController` 0))
  (bind _childactor (`ChildActorComponent.ChildActor` (`self.BP-Tank1Model`)))
  (`PlayerController.SetViewTargetWithBlend` (`GameplayStatics.GetPlayerController` 0) _childactor 0.0 "VTBlend_Linear" 0.0 false) ; Use child actor's camera
  (bind _asbp_tank_base (cast `/Game/Blueprint/TankModels/BP-TankBase` _childactor))
  (set `self.Tank Controller` _asbp_tank_base)
  (`/Engine/EditorBlueprintResources/StandardMacros.IsValid` _returnvalue
    (:`Is Valid`
      (`EnhancedInputSubsystemInterface.AddMappingContext` (pcsubsystem `EnhancedInputLocalPlayerSubsystem` _returnvalue) "/Game/Blueprint/Input/IMC_Player.IMC_Player" 0 (struct))
      (bind _springarm (`/Game/Blueprint/TankModels/BP-TankBase.Get Camera Spring Arm` (`self.Tank Controller`)))
      (bind _output_get (set `self.Spring Arm` _springarm))
      (set `self.Camera Rotation` (`SceneComponent.RelativeRotation` _output_get))
      (bind _returnvalue_2 (`|CreateWidget` "/Game/UI/WBP_PlayerHUD.WBP_PlayerHUD_C" (`GameplayStatics.GetPlayerController` 0)))
      (bind _output_get_2 (set `self.Player HUD` _returnvalue_2))
      (`UserWidget.AddToViewport` _output_get_2 0)
      (`self.Update Health`)
      (bind _asgm_main (cast `/Game/Blueprint/GM_Main` (`GameplayStatics.GetGameMode`)))
      (`self.Set Remaining Enemies` (`KismetArrayLibrary.Array_Length` (`/Game/Blueprint/GM_Main.Remaining Enemies` _asgm_main))))))

(event `self.ReceiveTick`
  (params (DeltaSeconds :type "Float (single-precision)"))
  (bind _tank_controller (`self.Tank Controller`))
  (bind (_worldposition _worlddirection) (`GameplayStatics.DeprojectScreenToWorld` (`GameplayStatics.GetPlayerController` 0) (/ (`WidgetLayoutLibrary.GetViewportSize`) 2.0)))
  (`/Game/Blueprint/TankModels/BP-TankBase.Update Upper Body Position` _tank_controller (`SceneComponent.RelativeRotation` (`/Game/Blueprint/TankModels/BP-TankBase.SpringArm` _tank_controller)))
  (`/Game/Blueprint/TankModels/BP-TankBase.Set Canon Pitch` (`self.Tank Controller`) (+ _worldposition (* _worlddirection 1000))))

(event `EnhancedInput|/Game/Blueprint/Input/IA_Look`
  (params (ActionValue :type "Vector2D Structure") (ElapsedSeconds :type "Float (double-precision)") (TriggeredSeconds :type "Float (double-precision)") (InputAction :type "InputAction Object Reference" :default "/Game/Blueprint/Input/IA_Look.IA_Look"))
  (bind (_camera_rotation_roll _camera_rotation_pitch _camera_rotation_yaw) (`KismetMathLibrary.BreakRotator` (`self.Camera Rotation`)))
  ; Camera
  (:`Triggered`
    (bind _output_get (set `self.Camera Rotation` (`KismetMathLibrary.MakeRotator` 0.0 (`KismetMathLibrary.FClamp` (+ (* ActionValue_Y (`self.Camera Y Sensitivity`)) _camera_rotation_pitch) -15.0 50.0) (+ (* ActionValue_X (`self.Camera X Sensitivity`)) _camera_rotation_yaw))))
    (`SceneComponent.K2_SetRelativeRotation` (`self.Spring Arm`) _output_get false false)))

(event `EnhancedInput|/Game/Blueprint/Input/IA_Throttle`
  (params (ActionValue :type "Float (double-precision)") (ElapsedSeconds :type "Float (double-precision)") (TriggeredSeconds :type "Float (double-precision)") (InputAction :type "InputAction Object Reference" :default "/Game/Blueprint/Input/IA_Throttle.IA_Throttle"))
  (bind _tank_controller (`self.Tank Controller`))
  ; Movement
  (:`Triggered`
    (set `/Game/Blueprint/TankModels/BP-TankBase.Throttle Input` ActionValue _tank_controller))
  (:`Completed`
    (set `/Game/Blueprint/TankModels/BP-TankBase.Throttle Input` 0.0 _tank_controller)))

(event `EnhancedInput|/Game/Blueprint/Input/IA_Steer`
  (params (ActionValue :type "Float (double-precision)") (ElapsedSeconds :type "Float (double-precision)") (TriggeredSeconds :type "Float (double-precision)") (InputAction :type "InputAction Object Reference" :default "/Game/Blueprint/Input/IA_Steer.IA_Steer"))
  (bind _tank_controller (`self.Tank Controller`))
  ; Movement
  (:`Triggered`
    (set `/Game/Blueprint/TankModels/BP-TankBase.Steer Input` ActionValue _tank_controller))
  (:`Completed`
    (set `/Game/Blueprint/TankModels/BP-TankBase.Steer Input` 0.0 _tank_controller)))

(event `EnhancedInput|/Game/Blueprint/Input/IA_Shoot`
  (params (ActionValue :type Boolean) (ElapsedSeconds :type "Float (double-precision)") (TriggeredSeconds :type "Float (double-precision)") (InputAction :type "InputAction Object Reference" :default "/Game/Blueprint/Input/IA_Shoot.IA_Shoot"))
  (:`Triggered`
    (bind (_hit_ _distance _hit_actor _shot_end) (`/Game/Blueprint/TankModels/BP-TankBase.Cast Cannon Shot` (`self.Tank Controller`)))
    (if _hit_
      (bind _asbp_tank_base (cast `/Game/Blueprint/TankModels/BP-TankBase` _hit_actor)
        (:`then`
          (`KismetSystemLibrary.Delay` (/ _distance (`self.Bullet Speed`)))
          (`/Engine/EditorBlueprintResources/StandardMacros.IsValid` _asbp_tank_base
            (:`Is Valid`
              (`KismetSystemLibrary.DrawDebugSphere` _shot_end 25.0 12 (struct :`R` 1.0 :`G` 1.0 :`B` 1.0 :`A` 1.0) 3.0)
              (bind _killed (`/Game/Blueprint/BC_Health.Apply Damage` (`/Game/Blueprint/TankModels/BP-TankBase.BC_Health` _asbp_tank_base) 1.0))
              (if _killed
                (`self.K2_DestroyActor` _hit_actor)))))
        (:`CastFailed`
          (`NiagaraFunctionLibrary.SpawnSystemAtLocation` "/Game/VFX/NS_DirtBlast.NS_DirtBlast" _shot_end (struct) (1.0 1.0 1.0) true true "AutoRelease"))))))

(fn `NewFunction`)

(fn `Set Remaining Enemies`
  (params (Amount :type Integer))
  (bind _player_hud (`self.Player HUD`))
  (`/Engine/EditorBlueprintResources/StandardMacros.IsValid` _player_hud
    (:`Is Valid`
      (`/Game/UI/WBP_PlayerHUD.Set Remining Enemies` _player_hud Amount))))

(fn `Update Health`
  (bind _percent (`/Game/Blueprint/BC_Health.Get Health Percentage` (`/Game/Blueprint/TankModels/BP-TankBase.BC_Health` (`self.Tank Controller`))))
  (`/Game/UI/WBP_PlayerHUD.Set Health` (`self.Player HUD`) _percent))

(fn `UserConstructionScript`)