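; BC_Health is a health component that tracks an actor's current and maximum health.
; It fills health to maximum on BeginPlay and exposes functions to apply damage, recover health capped at the maximum, and report the health fraction.
; Applying damage sends an OnDmgTaken message to the owner and returns whether health has dropped to zero or below, leaving death handling outside the component.
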(event `self.ReceiveBeginPlay`
  (set `self.Current Health` (`self.Max Health`)))

(event `On Dmg Taken`)

(fn `Apply Damage`
  (params (Damage :type "Float (double-precision)"))
  (returns (Killed :type Boolean))
  (bind _output_get (set `self.Current Health` (- (`self.Current Health`) Damage)))
  (message `/Game/Blueprint/BPI_HealthEvents.On Dmg Taken` (`self.GetOwner`))
  (if (<= _output_get 0.0)
    (return true)
    (else
      (return false))))

(fn `Get Health Percentage`
  (returns (Percent :type "Float (double-precision)"))
  (return (/ (`self.Current Health`) (`self.Max Health`))))

(fn `Recover Health`
  (params (Amount :type "Float (double-precision)"))
  (bind _returnvalue (+ Amount (`self.Current Health`)))
  (if (> _returnvalue (`self.Max Health`))
    (set `self.Current Health` (`self.Max Health`))
    (else
      (set `self.Current Health` _returnvalue)))
  (return))