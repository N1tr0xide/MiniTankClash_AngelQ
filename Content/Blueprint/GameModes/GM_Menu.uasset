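; Game mode for the main menu, driving its cameras and spawning the menu widget.
; On BeginPlay it views MainCam, then, if a CamRig-tagged rail exists, shows WBP_Menu with the mouse cursor and animates the rail position via a timeline.
; How-to-play enter and exit events blend between HowToCam and MainCam through SwitchToCam, which finds targets by actor tag and uses cubic blending.
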(event `self.ReceiveBeginPlay`
  (bind _returnvalue (`GameplayStatics.GetPlayerController` 0))
  (`self.Switch To Cam` "MainCam")
  (bind _outactors (`GameplayStatics.GetAllActorsWithTag` "CamRig"))
  (bind _output (`|GetArrayItem` _outactors))
  (`/Engine/EditorBlueprintResources/StandardMacros.IsValid` _output
    (:`Is Valid`
      (bind _ascamera_rig_rail (cast `CameraRig_Rail` _output))
      (set `self.Camera Rig Rail` _ascamera_rig_rail)
      (bind _returnvalue_2 (`|CreateWidget` "/Game/UI/WBP_Menu.WBP_Menu_C" _returnvalue))
      (`UserWidget.AddToViewport` _returnvalue_2 0)
      (set `PlayerController.bShowMouseCursor` true _returnvalue)
      (bind (_direction _rig_position) (`Timeline|Timeline` :!via `PlayFromStart`)
        (:`Update`
          (set `CameraRig_Rail.CurrentPositionOnRail` _rig_position (`self.Camera Rig Rail`)))))))

(event `/Game/Blueprint/BPI_GMenuComms.On How To Play Enter`
  (`self.Switch To Cam` "HowToCam" 0.5))

(event `/Game/Blueprint/BPI_GMenuComms.On How to Play Exit`
  (`self.Switch To Cam` "MainCam" 0.5))

(fn `Switch To Cam`
  (params (Tag :type Name) (`Blend Time` :type "Float (double-precision)"))
  (bind _outactors (`GameplayStatics.GetAllActorsWithTag` Tag))
  (`PlayerController.SetViewTargetWithBlend` (`GameplayStatics.GetPlayerController` 0) (`|GetArrayItem` _outactors) `Blend Time` "VTBlend_Cubic" 3.0 false))

(fn `UserConstructionScript`)