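; GM_Main is the game mode that tracks remaining enemies and runs the win and lose endings.
; Registering an enemy adds it to a list, spawns its health marker widget and updates the player's count; unregistering updates the HUD and triggers victory when none remain.
; Victory animates global time dilation on a timeline before switching to the tank's front camera and showing the win screen.
; Defeat blends to the first CameraActor found and shows the lose screen.
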(event `/Game/Blueprint/BPI_GMComms.On Game Win`
  (bind _returnvalue (`GameplayStatics.GetPlayerController` 0))
  (bind _asbp_player (cast `/Game/Blueprint/BP_Player` (`GameplayStatics.GetPlayerPawn` 0))
    (:`then`
      (bind (_direction _time_scale) (`Timeline|Timeline` :!via `PlayFromStart`)
        (:`Update`
          (`GameplayStatics.SetGlobalTimeDilation` _time_scale))
        (:`Finished`
          (`/Game/Blueprint/TankModels/BP-TankBase.Get Front Cam` (`/Game/Blueprint/BP_Player.Tank Controller` _asbp_player))
          (`WidgetLayoutLibrary.RemoveAllWidgets`)
          (set `PlayerController.bShowMouseCursor` true _returnvalue)
          (bind _returnvalue_2 (`|CreateWidget` "/Game/UI/WBP_GameWin.WBP_GameWin_C" _returnvalue))
          (`UserWidget.AddToViewport` _returnvalue_2 0))))
    (:`CastFailed`
      (`KismetSystemLibrary.PrintString` "Player Cast GM Failure"))))

(event `/Game/Blueprint/BPI_GMComms.On Game Over`
  (bind _returnvalue (`GameplayStatics.GetPlayerController` 0))
  (bind _outactors (`GameplayStatics.GetAllActorsOfClass` "/Script/Engine.CameraActor"))
  (`PlayerController.SetViewTargetWithBlend` (`GameplayStatics.GetPlayerController` 0) (`|GetArrayItem` _outactors) 0.25 "VTBlend_Linear" 0.0 false)
  (`WidgetLayoutLibrary.RemoveAllWidgets`)
  (set `PlayerController.bShowMouseCursor` true _returnvalue)
  (bind _returnvalue_2 (`|CreateWidget` "/Game/UI/WBP_GameLost.WBP_GameLost_C" _returnvalue))
  (`UserWidget.AddToViewport` _returnvalue_2 0))

(fn `RegisterEnemy`
  (params (Actor :type "Actor Object Reference"))
  (returns (`Health Widget` :type "/Game/UI/WBP_EnemyHealthMarker Object Reference"))
  (`KismetArrayLibrary.Array_Add` (`self.Remaining Enemies`) Actor)
  (bind _returnvalue (`|CreateWidget` "/Game/UI/WBP_EnemyHealthMarker.WBP_EnemyHealthMarker_C" (`GameplayStatics.GetPlayerController` 0)))
  (`UserWidget.AddToViewport` _returnvalue 0)
  (bind _asbp_player (cast `/Game/Blueprint/BP_Player` (`GameplayStatics.GetPlayerPawn` 0))
    (:`then`
      (`/Game/Blueprint/BP_Player.Set Remaining Enemies` _asbp_player (`KismetArrayLibrary.Array_Length` (`self.Remaining Enemies`))))
    (:`CastFailed`
      _))
  (return _returnvalue))

(fn `UnregisterEnemy`
  (params (Actor :type "Actor Object Reference"))
  (bind _returnvalue (`KismetArrayLibrary.Array_Length` (`self.Remaining Enemies`)))
  (if (`KismetArrayLibrary.Array_Contains` (`self.Remaining Enemies`) Actor)
    (`KismetArrayLibrary.Array_RemoveItem` (`self.Remaining Enemies`) Actor)
    (bind _asbp_player (cast `/Game/Blueprint/BP_Player` (`GameplayStatics.GetPlayerPawn` 0)))
    (`/Game/UI/WBP_PlayerHUD.Set Remining Enemies` (`/Game/Blueprint/BP_Player.Player HUD` _asbp_player) _returnvalue)
    (if (<= _returnvalue 0)
      (`self.On Game Win`))))

(fn `UserConstructionScript`)