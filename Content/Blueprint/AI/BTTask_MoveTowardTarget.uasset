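; Behavior tree task that drives an AI-controlled BP-TankBase toward a point at a blackboard-set distance from its target actor.
; Execute caches the tank and blackboard; Tick writes the target's location to the blackboard and debug-draws the standoff point.
; Dot products of the tank's forward and right vectors with the direction to that point set throttle and steering, zeroed when close.
; A tick with a valid target finishes the task successfully, even before arrival.
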(event `self.ReceiveExecute`
  (params (OwnerActor :type "Actor Object Reference"))
  (bind _asbp_tank_base (cast `/Game/Blueprint/TankModels/BP-TankBase` (`Controller.K2_GetPawn` (`AIBlueprintHelperLibrary.GetAIController` OwnerActor))))
  (set `self.BPBase - Tank` _asbp_tank_base)
  (set `self.Blackboard` (`AIBlueprintHelperLibrary.GetBlackboard` OwnerActor)))

(event `self.ReceiveTick`
  (params (OwnerActor :type "Actor Object Reference") (DeltaSeconds :type "Float (single-precision)"))
  (bind _bpbase___tank (`self.BPBase - Tank`))
  (bind _bpbase___tank_2 (`self.BPBase - Tank`))
  (bind _blackboard (`self.Blackboard`))
  (bind _returnvalue (`BlackboardComponent.GetValueAsObject` _blackboard (`self.target actor Key`)))
  (bind _rootcomponent (`Actor.RootComponent` (`self.BPBase - Tank`)))
  (bind _returnvalue_2 (`SceneComponent.K2_GetComponentLocation` _rootcomponent))
  (`/Engine/EditorBlueprintResources/StandardMacros.IsValid` _returnvalue
    (:`Is Valid`
      (bind _asactor (cast `Actor` _returnvalue))
      (bind _returnvalue_3 (`SceneComponent.K2_GetComponentLocation` (`Actor.RootComponent` _asactor)))
      (`BlackboardComponent.SetValueAsVector` _blackboard (`self.target Location Key`) _returnvalue_3) ; update target pos
      (bind _returnvalue_4 (+ _returnvalue_3 (* (`KismetMathLibrary.Normal` (- (`SceneComponent.K2_GetComponentLocation` (`Actor.RootComponent` (`self.BPBase - Tank`))) _returnvalue_3)) (`BlackboardComponent.GetValueAsFloat` _blackboard (`self.desired distance Key`)))))
      (`KismetSystemLibrary.DrawDebugSphere` _returnvalue_4 10.0 12 (struct :`R` 1.0 :`G` 0.956479 :`B` 0.494777 :`A` 1.0))
      ; Update Inputs
      (if (> (`KismetMathLibrary.Vector_Distance` _returnvalue_2 _returnvalue_4) 50.0)
        (bind _returnvalue_5 (`KismetMathLibrary.Normal` (- _returnvalue_4 _returnvalue_2)))
        (set `/Game/Blueprint/TankModels/BP-TankBase.Throttle Input` (`KismetMathLibrary.FClamp` (`KismetMathLibrary.Dot_VectorVector` (`SceneComponent.GetForwardVector` _rootcomponent) _returnvalue_5) -1.0) _bpbase___tank)
        (set `/Game/Blueprint/TankModels/BP-TankBase.Steer Input` (`KismetMathLibrary.FClamp` (`KismetMathLibrary.Dot_VectorVector` (`SceneComponent.GetRightVector` _rootcomponent) _returnvalue_5) -1.0) _bpbase___tank)
        (else
          (set `/Game/Blueprint/TankModels/BP-TankBase.Throttle Input` 0.0 _bpbase___tank_2)
          (set `/Game/Blueprint/TankModels/BP-TankBase.Steer Input` 0.0 _bpbase___tank_2)))
      (`self.FinishExecute` true))))