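; Behavior Tree task that pitches an AI tank's cannon toward a target location and records whether it has line of sight to the player.
; On execute it caches the controlled BP-TankBase pawn and the Blackboard.
; On tick it passes the Blackboard target to SetCanonPitch, sets the line-of-sight key by whether the returned actor is tagged Player, then finishes successfully.
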(event `self.ReceiveExecute`
  (params (OwnerActor :type "Actor Object Reference"))
  (bind _asbp_tank_base (cast `/Game/Blueprint/TankModels/BP-TankBase` (`Controller.K2_GetPawn` (`AIBlueprintHelperLibrary.GetAIController` OwnerActor))))
  (set `self.BPBase - Tank` _asbp_tank_base)
  (set `self.Blackboard` (`AIBlueprintHelperLibrary.GetBlackboard` OwnerActor)))

(event `self.ReceiveTick`
  (params (OwnerActor :type "Actor Object Reference") (DeltaSeconds :type "Float (single-precision)"))
  (bind _hitactor (`/Game/Blueprint/TankModels/BP-TankBase.Set Canon Pitch` (`self.BPBase - Tank`) (`BlackboardComponent.GetValueAsVector` (`self.Blackboard`) (`self.target Location Key`))))
  (`/Engine/EditorBlueprintResources/StandardMacros.IsValid` _hitactor
    (:`Is Valid`
      (`BlackboardComponent.SetValueAsBool` (`self.Blackboard`) (`self.hasLineOfSight Key`) (`Actor.ActorHasTag` _hitactor "Player")))
    (:`Is Not Valid`
      (`BlackboardComponent.SetValueAsBool` (`self.Blackboard`) (`self.hasLineOfSight Key`) false)))
  (`self.FinishExecute` true))