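; Behavior Tree task that drives an AI tank toward its blackboard target along a navmesh path around obstacles.
; On execute it saves the target's location to the blackboard and finds a synchronous path to a point offset by a separation distance.
; Tick converts dot products toward the current waypoint into throttle and steering, advancing when close.
; It finishes successfully after setting inputs or passing the last point, and fails without a path.
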(event `self.ReceiveExecute`
  (params (OwnerActor :type "Actor Object Reference"))
  (bind _blackboard (`self.Blackboard`))
  (bind _returnvalue (`BlackboardComponent.GetValueAsObject` _blackboard (`self.target actor Key`)))
  (bind _returnvalue_2 (`SceneComponent.K2_GetComponentLocation` (`Actor.RootComponent` (`self.BPBase - Tank`))))
  (bind _asbp_tank_base (cast `/Game/Blueprint/TankModels/BP-TankBase` (`Controller.K2_GetPawn` (`AIBlueprintHelperLibrary.GetAIController` OwnerActor))))
  (set `self.BPBase - Tank` _asbp_tank_base)
  (set `self.Blackboard` (`AIBlueprintHelperLibrary.GetBlackboard` OwnerActor))
  (`/Engine/EditorBlueprintResources/StandardMacros.IsValid` _returnvalue
    (:`Is Valid`
      (bind _asactor (cast `Actor` _returnvalue))
      (bind _returnvalue_3 (`SceneComponent.K2_GetComponentLocation` (`Actor.RootComponent` _asactor)))
      (`BlackboardComponent.SetValueAsVector` _blackboard (`self.target Location Key`) _returnvalue_3) ; update target's pos
      (bind _returnvalue_4 (`NavigationSystemV1.FindPathToLocationSynchronously` _returnvalue_2 (+ _returnvalue_3 (* (`KismetMathLibrary.Normal` (- _returnvalue_2 _returnvalue_3)) (`self.Separation to Target`))) null null)) ; find path around obstacles
      (bind _output_get (set `self.Path Points` (`NavigationPath.PathPoints` _returnvalue_4)))
      (set `self.Current Path Index` 0)
      (for _array_element _output_get
        _))))

(event `self.ReceiveTick`
  (params (OwnerActor :type "Actor Object Reference") (DeltaSeconds :type "Float (single-precision)"))
  (bind _bpbase___tank (`self.BPBase - Tank`))
  (bind _path_points (`self.Path Points`))
  (bind _output (`|GetArrayItem` _path_points (`self.Current Path Index`)))
  (bind _rootcomponent (`Actor.RootComponent` (`self.BPBase - Tank`)))
  (bind _returnvalue (`SceneComponent.K2_GetComponentLocation` _rootcomponent))
  (bind _returnvalue_2 (`KismetMathLibrary.Normal` (- _output _returnvalue)))
  (if (> (`KismetArrayLibrary.Array_Length` _path_points) 0)
    ; Update Inputs
    (if (> (`KismetMathLibrary.Vector_Distance` _returnvalue _output) 20.0)
      (set `/Game/Blueprint/TankModels/BP-TankBase.Throttle Input` (`KismetMathLibrary.FClamp` (`KismetMathLibrary.Dot_VectorVector` (`SceneComponent.GetForwardVector` _rootcomponent) _returnvalue_2) -1.0) _bpbase___tank)
      (set `/Game/Blueprint/TankModels/BP-TankBase.Steer Input` (`KismetMathLibrary.FClamp` (`KismetMathLibrary.Dot_VectorVector` (`SceneComponent.GetRightVector` _rootcomponent) _returnvalue_2) -1.0) _bpbase___tank)
      (`self.FinishExecute` true :!label _label)
      (else
        (bind _output_get (set `self.Current Path Index` (+ (`self.Current Path Index`) 1)))
        (if (>= _output_get (`KismetArrayLibrary.Array_Length` (`self.Path Points`)))
          (goto _label))))
    (else
      (`self.FinishExecute` false))))