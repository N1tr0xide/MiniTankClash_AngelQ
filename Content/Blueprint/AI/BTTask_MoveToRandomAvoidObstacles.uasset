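; Behavior Tree task that drives an AI tank to a random reachable point nearby, following a navmesh path around obstacles.
; On execute it picks a point within a radius, offsets it toward the tank by a separation distance, then stores and debug-draws the path.
; Each tick it sets throttle and steering from forward and right dot products toward the current waypoint, advancing when close and finishing after the last.
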(event `self.ReceiveExecute`
  (params (OwnerActor :type "Actor Object Reference"))
  (bind _returnvalue (`SceneComponent.K2_GetComponentLocation` (`Actor.RootComponent` (`self.BPBase - Tank`))))
  (bind (_randomlocation _returnvalue_2) (`NavigationSystemV1.K2_GetRandomReachablePointInRadius` _returnvalue (`self.Random Point Radius`) null null))
  (bind _asbp_tank_base (cast `/Game/Blueprint/TankModels/BP-TankBase` (`Controller.K2_GetPawn` (`AIBlueprintHelperLibrary.GetAIController` OwnerActor))))
  (set `self.BPBase - Tank` _asbp_tank_base)
  (set `self.Blackboard` (`AIBlueprintHelperLibrary.GetBlackboard` OwnerActor))
  (if _returnvalue_2
    (bind _returnvalue_3 (`NavigationSystemV1.FindPathToLocationSynchronously` _returnvalue (+ _randomlocation (* (`KismetMathLibrary.Normal` (- _returnvalue _randomlocation)) (`self.Separation to Target`))) null null)) ; find path around obstacles
    (bind _output_get (set `self.Path Points` (`NavigationPath.PathPoints` _returnvalue_3)))
    (set `self.Current Path Index` 0)
    (for _array_element _output_get
      (`KismetSystemLibrary.DrawDebugSphere` _array_element 30.0 12 (struct :`R` 1.0 :`B` 0.033869 :`A` 1.0) 10.0))))

(event `self.ReceiveTick`
  (params (OwnerActor :type "Actor Object Reference") (DeltaSeconds :type "Float (single-precision)"))
  (bind _bpbase___tank (`self.BPBase - Tank`))
  (bind _output (`|GetArrayItem` (`self.Path Points`) (`self.Current Path Index`)))
  (bind _rootcomponent (`Actor.RootComponent` (`self.BPBase - Tank`)))
  (bind _returnvalue (`SceneComponent.K2_GetComponentLocation` _rootcomponent))
  (bind _returnvalue_2 (`KismetMathLibrary.Normal` (- _output _returnvalue)))
  ; Update Inputs
  (if (> (`KismetMathLibrary.Vector_Distance` _returnvalue _output) 20.0)
    (set `/Game/Blueprint/TankModels/BP-TankBase.Throttle Input` (`KismetMathLibrary.FClamp` (`KismetMathLibrary.Dot_VectorVector` (`SceneComponent.GetForwardVector` _rootcomponent) _returnvalue_2) -1.0) _bpbase___tank)
    (set `/Game/Blueprint/TankModels/BP-TankBase.Steer Input` (`KismetMathLibrary.FClamp` (`KismetMathLibrary.Dot_VectorVector` (`SceneComponent.GetRightVector` _rootcomponent) _returnvalue_2) -1.0) _bpbase___tank)
    (else
      (bind _output_get (set `self.Current Path Index` (+ (`self.Current Path Index`) 1)))
      (if (>= _output_get (`KismetArrayLibrary.Array_Length` (`self.Path Points`)))
        (`self.FinishExecute` true)))))