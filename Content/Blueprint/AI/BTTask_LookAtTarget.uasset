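; Behavior tree task that aims an AI tank's upper body at a target location stored in the Blackboard.
; On execute it caches the controlled BP-TankBase pawn and the Blackboard.
; On Tick it passes the look-at rotation from the upper body rotator to that location into UpdateUpperBodyPosition, then finishes successfully without waiting for alignment.
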(event `self.ReceiveExecute`
  (params (OwnerActor :type "Actor Object Reference"))
  (bind _asbp_tank_base (cast `/Game/Blueprint/TankModels/BP-TankBase` (`Controller.K2_GetPawn` (`AIBlueprintHelperLibrary.GetAIController` OwnerActor))))
  (set `self.BPBase - Tank` _asbp_tank_base)
  (set `self.Blackboard` (`AIBlueprintHelperLibrary.GetBlackboard` OwnerActor)))

(event `self.ReceiveTick`
  (params (OwnerActor :type "Actor Object Reference") (DeltaSeconds :type "Float (single-precision)"))
  (bind _bpbase___tank (`self.BPBase - Tank`))
  (`/Game/Blueprint/TankModels/BP-TankBase.Update Upper Body Position` _bpbase___tank (`KismetMathLibrary.FindLookAtRotation` (`SceneComponent.K2_GetComponentLocation` (`/Game/Blueprint/TankModels/BP-TankBase.Upper Body Rotator` _bpbase___tank)) (`BlackboardComponent.GetValueAsVector` (`self.Blackboard`) (`self.target Location Key`))))
  (`self.FinishExecute` true))