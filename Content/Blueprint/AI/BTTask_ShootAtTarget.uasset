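; Behavior tree task that makes an AI-controlled tank shoot at the blackboard target actor.
; Each tick it accumulates a timer while the shoot point's aim stays within an angle threshold, then traces a cannon shot.
; Tank hits wait a distance-over-speed delay to simulate travel, then explode and apply damage, possibly destroying the victim.
; Other hits spawn a dirt blast; the task finishes once a hit resolves.
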(event `self.ReceiveExecute`
  (params (OwnerActor :type "Actor Object Reference"))
  (bind _returnvalue (`BlackboardComponent.GetValueAsObject` (`self.Blackboard`) (`self.target actor Key`)))
  (bind _asbp_tank_base (cast `/Game/Blueprint/TankModels/BP-TankBase` (`Controller.K2_GetPawn` (`AIBlueprintHelperLibrary.GetAIController` OwnerActor))))
  (set `self.BPBase - Tank` _asbp_tank_base)
  (set `self.Blackboard` (`AIBlueprintHelperLibrary.GetBlackboard` OwnerActor))
  (`/Engine/EditorBlueprintResources/StandardMacros.IsValid` _returnvalue
    (:`Is Valid`
      (bind _asactor (cast `Actor` _returnvalue))
      (set `self.Target Actor` (`Actor.RootComponent` _asactor)))))

(event `self.ReceiveTick`
  (params (OwnerActor :type "Actor Object Reference") (DeltaSeconds :type "Float (single-precision)"))
  (set `self.Delta Seconds` DeltaSeconds)
  (bind (_is_valid _angle) (`self.Get Angle To Actor` (`self.Target Actor`)))
  (if _is_valid
    (if (<= _angle (`self.Max Angle for Shot`))
      (bind _output_get (set `self.TImer` (+ (`self.TImer`) (`self.Delta Seconds`))))
      (if (>= _output_get (`self.Shot Timer Threshold`))
        (set `self.TImer` 0.0)
        (bind (_hit_ _distance _hit_actor _shot_end _impactnormal) (`/Game/Blueprint/TankModels/BP-TankBase.Cast Cannon Shot` (`self.BPBase - Tank`)))
        (if _hit_
          (bind _asbp_tank_base (cast `/Game/Blueprint/TankModels/BP-TankBase` _hit_actor)
            (:`then`
              (`KismetSystemLibrary.Delay` (/ _distance (`self.Bullet Speed`)))
              (`/Engine/EditorBlueprintResources/StandardMacros.IsValid` _asbp_tank_base
                (:`Is Valid`
                  (`GameplayStatics.SpawnEmitterAtLocation` "/Game/VFX/M5VFXVOL2/Particles/Explosion/Fire_Exp_00.Fire_Exp_00" _shot_end (`KismetMathLibrary.MakeRotFromX` _impactnormal) (0.1 0.1 0.1) true "AutoRelease")
                  (bind _killed (`/Game/Blueprint/BC_Health.Apply Damage` (`/Game/Blueprint/TankModels/BP-TankBase.BC_Health` _asbp_tank_base) 1.0))
                  (if _killed
                    (`Actor.K2_DestroyActor` _hit_actor)))))
            (:`CastFailed`
              (`NiagaraFunctionLibrary.SpawnSystemAtLocation` "/Game/VFX/NS_DirtBlast.NS_DirtBlast" _shot_end (struct) (1.0 1.0 1.0) true true "AutoRelease")))
          (`self.FinishExecute` true)))
      (else
        (set `self.TImer` 0.0 :!label _label)))
    (else
      (goto _label))))

(fn `Get Angle To Actor`
  (params (Target :type "SceneComponent Object Reference"))
  (returns (`Is Valid` :type Boolean) (Angle :type "Float (double-precision)"))
  (`/Engine/EditorBlueprintResources/StandardMacros.IsValid` Target
    (:`Is Valid`
      (return true (`KismetMathLibrary.DegAcos` (`KismetMathLibrary.Dot_VectorVector` (`KismetMathLibrary.Normal` (`SceneComponent.GetForwardVector` (`/Game/Blueprint/TankModels/BP-TankBase.Shoot Point` (`self.BPBase - Tank`)))) (`KismetMathLibrary.Normal` (- (`SceneComponent.K2_GetComponentLocation` Target) (`SceneComponent.K2_GetComponentLocation` (`/Game/Blueprint/TankModels/BP-TankBase.Shoot Point` (`self.BPBase - Tank`)))))))))
    (:`Is Not Valid`
      (return false 0.0))))