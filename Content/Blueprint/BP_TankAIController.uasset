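; AI controller for enemy tanks that runs the BT_TankAI behavior tree on possession and seeds the desired separation distance into the blackboard.
; AI perception sets any perceived BP-TankBase tagged "Player" as the blackboard target, and clears it when perception forgets a target.
; An unconnected debug sphere draw around the controlled pawn is left in the graph.
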(event `self.ReceivePossess`
  (params (PossessedPawn :type "Pawn Object Reference"))
  (`self.RunBehaviorTree` "/Game/Blueprint/AI/BT_TankAI.BT_TankAI")
  (`BlackboardComponent.SetValueAsFloat` (`AIBlueprintHelperLibrary.GetBlackboard` null) (`self.desired separation Key`) (`self.Desired Separation From Target`)))

(event `self.AIPerception.OnTargetPerceptionUpdated`
  (params (Actor :type "Actor Object Reference") (Stimulus :type "AIStimulus Structure"))
  (bind _asbp_tank_base (cast `/Game/Blueprint/TankModels/BP-TankBase` Actor))
  (if (`self.ActorHasTag` _asbp_tank_base "Player")
    (`BlackboardComponent.SetValueAsObject` (`AIBlueprintHelperLibrary.GetBlackboard` null) (`self.target actor key`) _asbp_tank_base)))

(event `self.AIPerception.OnTargetPerceptionForgotten`
  (params (Actor :type "Actor Object Reference"))
  (`BlackboardComponent.SetValueAsObject` (`AIBlueprintHelperLibrary.GetBlackboard` null) (`self.target actor key`) null))

(event `self.ReceiveTick`
  (params (DeltaSeconds :type "Float (single-precision)")))

(fn `UserConstructionScript`)