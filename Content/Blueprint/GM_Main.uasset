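; GM_Main, likely the main game mode, tracks the remaining enemies and keeps the player's enemy count current.
; RegisterEnemy stores the actor, creates an on-screen WBP_EnemyHealthMarker, sends the new count to BP_Player and returns the widget to the caller.
; UnregisterEnemy removes a tracked actor and writes the count straight to the player's HUD, without touching the marker widget.
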(fn `RegisterEnemy`
  (params (Actor :type "Actor Object Reference"))
  (returns (`Health Widget` :type "/Game/UI/WBP_EnemyHealthMarker Object Reference"))
  (`KismetArrayLibrary.Array_Add` (`self.Remaining Enemies`) Actor)
  (bind _returnvalue (`|CreateWidget` "/Game/UI/WBP_EnemyHealthMarker.WBP_EnemyHealthMarker_C" (`GameplayStatics.GetPlayerController` 0)))
  (`UserWidget.AddToViewport` _returnvalue 0)
  (bind _asbp_player (cast `/Game/Blueprint/BP_Player` (`GameplayStatics.GetPlayerPawn` 0))
    (:`then`
      (`/Game/Blueprint/BP_Player.Set Remaining Enemies` _asbp_player (`KismetArrayLibrary.Array_Length` (`self.Remaining Enemies`))))
    (:`CastFailed`
      _))
  (return _returnvalue))

(fn `UnregisterEnemy`
  (params (Actor :type "Actor Object Reference"))
  (if (`KismetArrayLibrary.Array_Contains` (`self.Remaining Enemies`) Actor)
    (`KismetArrayLibrary.Array_RemoveItem` (`self.Remaining Enemies`) Actor)
    (bind _asbp_player (cast `/Game/Blueprint/BP_Player` (`GameplayStatics.GetPlayerPawn` 0)))
    (`/Game/UI/WBP_PlayerHUD.Set Remining Enemies` (`/Game/Blueprint/BP_Player.Player HUD` _asbp_player) (`KismetArrayLibrary.Array_Length` (`self.Remaining Enemies`)))))

(fn `UserConstructionScript`)